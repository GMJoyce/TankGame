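; BP_TankProjectile is a tank shell that resolves everything in its sphere's hit event.
; Every impact spawns a large explosion, and a struck BP_Tank is pushed along the shell's velocity.
; A hit on the player's tank hides both and reloads BattleGround after a short delay.
; Another tank is destroyed with the shell after triggering SlowMo on the player's tank; other hits just destroy the shell.
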(event `self.ReceiveTick`
  (params (DeltaSeconds :type "Float (single-precision)")))

(event `self.Sphere.OnComponentHit`
  (params (HitComponent :type "PrimitiveComponent Object Reference") (OtherActor :type "Actor Object Reference") (OtherComp :type "PrimitiveComponent Object Reference") (NormalImpulse :type "Vector Structure") (Hit :type "HitResult Structure (by ref)"))
  (bind _returnvalue (`Controller.K2_GetPawn` (`GameplayStatics.GetPlayerController` 0)))
  (`GameplayStatics.SpawnEmitterAtLocation` "/Game/StarterContent/Particles/P_Explosion.P_Explosion" (+ (`self.K2_GetActorLocation`) (0.0 0.0 100.0)) (struct) (8.0 8.0 8.0))
  (bind _asbp_tank (cast `/Game/Blueprint/Tank/BP_Tank` OtherActor)
    (:`then`
      (`PrimitiveComponent.AddForce` (`/Game/Blueprint/Tank/BP_Tank.TankBody` _asbp_tank) (* (`self.GetVelocity`) 50.0) "None" true)
      (if (== (`Controller.K2_GetPawn` (`Pawn.GetController` _asbp_tank)) _returnvalue)
        (`self.SetActorHiddenInGame` _asbp_tank true)
        (`self.SetActorHiddenInGame` true)
        (`KismetSystemLibrary.Delay` 1.0)
        (`GameplayStatics.OpenLevel` "BattleGround")
        (else
          (`|ExecutionSequence`
            (:`then_0`
              (bind _asbp_tank_2 (cast `/Game/Blueprint/Tank/BP_Tank` _returnvalue))
              (`/Game/Blueprint/Tank/BP_Tank.SlowMo` _asbp_tank_2))
            (:`then_1`
              (`self.K2_DestroyActor` _asbp_tank)
              (`self.K2_DestroyActor`))))))
    (:`CastFailed`
      (`self.K2_DestroyActor`))))

(fn `UserConstructionScript`)