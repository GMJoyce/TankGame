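; BP_Tank is the player tank Blueprint, which here implements only camera look controls.
; AimAzimuth and AimElevation axis inputs drive controller yaw and pitch, scaled by world delta seconds and a fixed rate.
; InvertXAxis and InvertYAxis flags set the sign of each axis and are toggled at runtime by the Multiply and Divide keys.
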(event `InputAxis|AimAzimuth`
  (params (AxisValue :type "Float (single-precision)"))
  ;[1 1 1 1 30] Camera Controls
  (`self.AddControllerYawInput` (* AxisValue (`GameplayStatics.GetWorldDeltaSeconds`) 75.0 (select `bool` (`self.Invert X Axis`) :`false` 1.0 :`true` -1.0 :!type "Float (single-precision)"))))

(event `InputAxis|AimElevation`
  (params (AxisValue :type "Float (single-precision)"))
  ;[1 1 1 1 30] Camera Controls
  (`self.AddControllerPitchInput` (* AxisValue (`GameplayStatics.GetWorldDeltaSeconds`) 75.0 (select `bool` (`self.Invert Y Axis`) :`false` -1.0 :`true` 1.0 :!type "Float (single-precision)"))))

(event `Key|Divide`
  (params (Key :type "Key Structure"))
  (:`Pressed`
    (set `self.Invert Y Axis` (not (`self.Invert Y Axis`)))))

(event `Key|Multiply`
  (params (Key :type "Key Structure"))
  (:`Pressed`
    (set `self.Invert X Axis` (not (`self.Invert X Axis`)))))

(fn `UserConstructionScript`)