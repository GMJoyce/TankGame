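; Player controller for a tank that puts the player's HUD on screen and handles quitting the game.
; On BeginPlay it creates a widget, hands it the controlled tank's TankAimingComponent and adds it to the viewport.
; The FoundAimingComponent event separately creates a PlayerUI widget from the component passed in, so UI setup exists on two paths.
; Pressing the Quit input action exits the game.
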(event `self.ReceiveBeginPlay`
  (bind _returnvalue (`|CreateWidget` "/Game/Blueprint/User_Interface/PlayerUI.PlayerUI_C"))
  (set `/Game/Blueprint/User_Interface/PlayerUI.BP Aiming Comp Reference` (`|GetArrayItem` (`self.K2_GetComponentsByClass` (`self.GetControlledTank`) "/Script/TankBattleGame.TankAimingComponent")) _returnvalue)
  (`UserWidget.AddToViewport` _returnvalue 0))

(event `InputAction|Quit`
  (params (Key :type "Key Structure"))
  (:`Pressed`
    (`KismetSystemLibrary.QuitGame` null "Quit")))

(event `self.FoundAimingComponent`
  (params (AimCompRef :type "TankAimingComponent Object Reference"))
  (bind _returnvalue (`|CreateWidget` "/Game/Blueprint/User_Interface/PlayerUI.PlayerUI_C"))
  (set `/Game/Blueprint/User_Interface/PlayerUI.BP Aiming Comp Reference` AimCompRef _returnvalue)
  (`UserWidget.AddToViewport` _returnvalue 0))

(fn `UserConstructionScript`)